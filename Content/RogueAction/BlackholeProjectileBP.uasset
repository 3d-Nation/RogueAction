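; Blackhole projectile Blueprint that collects overlapped actors and destroys them when a fixed timer expires.
; On BeginPlay its sphere component ignores the instigator during movement and a one-shot timer starts.
; Sphere overlaps add actors uniquely to HitActor.
; On expiry it destroys each stored actor and calls its own destruction inside that loop, so an empty list leaves the projectile alive.
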(event OnComponentBeginOverlap(SphereComp)
  (params (OverlappedComponent :type Primitive%20Component%20Object%20Reference) (OtherActor :type Actor%20Object%20Reference) (OtherComp :type Primitive%20Component%20Object%20Reference) (OtherBodyIndex :type Integer) (bFromSweep :type Boolean) (SweepResult :type Hit%20Result%20Structure%20%28by%20ref%29))
  (Utilities|Array|AddUnique (Variables|Default|GetHitActor) OtherActor))

(event Custom|TimerElapsed
  (for _array_element (Variables|Default|GetHitActor)
    (Actor|DestroyActor _array_element)
    (Actor|DestroyActor)))

(event EventBeginPlay
  (Collision|IgnoreActorwhenMoving (Variables|Default|GetSphereComp) (Game|GetInstigator) true)
  (Utilities|Time|SetTimerbyEvent (delegate Custom|TimerElapsed) 4.7))

(fn ConstructionScript)